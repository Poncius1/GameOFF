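; Simon Says minigame actor where the player repeats a random sequence of four colored lights.
; Using the main trigger sets note count and speed from Difficulty, builds the sequence, and flashes it through a delayed self-calling event.
; Overlap-driven gates route Use presses to each color, where CheckNote compares the input.
; Mistakes flash red and reset Difficulty; completed sequences raise it, printing a win message at MaxLevel.
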(event OnComponentBeginOverlap(Trigger)
  (params (OverlappedComponent :type Primitive%20Component%20Object%20Reference) (OtherActor :type Actor%20Object%20Reference) (OtherComp :type Primitive%20Component%20Object%20Reference) (OtherBodyIndex :type Integer) (bFromSweep :type Boolean) (SweepResult :type Hit%20Result%20Structure%20%28by%20ref%29))
  ;[1 1 1] PlayerTrigger Overlap Events
  (Utilities|Casting|CastToThirdPersonCharacter OtherActor)
  (Input|EnableInput (Game|GetPlayerController 0))
  (Utilities|FlowControl|Gate true) ; enters at Open
)

(event OnComponentEndOverlap(Trigger)
  (params (OverlappedComponent :type Primitive%20Component%20Object%20Reference) (OtherActor :type Actor%20Object%20Reference) (OtherComp :type Primitive%20Component%20Object%20Reference) (OtherBodyIndex :type Integer))
  ;[1 1 1] PlayerTrigger Overlap Events
  (Utilities|Casting|CastToThirdPersonCharacter OtherActor)
  (Input|DisableInput (Game|GetPlayerController 0))
  (Utilities|FlowControl|Gate true) ; enters at Close
)

(event OnComponentBeginOverlap(Red_Trigger)
  (params (OverlappedComponent :type Primitive%20Component%20Object%20Reference) (OtherActor :type Actor%20Object%20Reference) (OtherComp :type Primitive%20Component%20Object%20Reference) (OtherBodyIndex :type Integer) (bFromSweep :type Boolean) (SweepResult :type Hit%20Result%20Structure%20%28by%20ref%29))
  ;[1 1 1] Listen To Player
  (Utilities|Casting|CastToThirdPersonCharacter OtherActor)
  (Input|EnableInput (Game|GetPlayerController 0))
  (Utilities|FlowControl|Gate true) ; enters at Open
)

(event OnComponentEndOverlap(Red_Trigger)
  (params (OverlappedComponent :type Primitive%20Component%20Object%20Reference) (OtherActor :type Actor%20Object%20Reference) (OtherComp :type Primitive%20Component%20Object%20Reference) (OtherBodyIndex :type Integer))
  ;[1 1 1] Listen To Player
  (Utilities|Casting|CastToThirdPersonCharacter OtherActor)
  (Input|DisableInput (Game|GetPlayerController 0))
  (Utilities|FlowControl|Gate true) ; enters at Close
)

(event OnComponentBeginOverlap(Green_Trigger)
  (params (OverlappedComponent :type Primitive%20Component%20Object%20Reference) (OtherActor :type Actor%20Object%20Reference) (OtherComp :type Primitive%20Component%20Object%20Reference) (OtherBodyIndex :type Integer) (bFromSweep :type Boolean) (SweepResult :type Hit%20Result%20Structure%20%28by%20ref%29))
  ;[1 1 1] Listen To Player
  (Utilities|Casting|CastToThirdPersonCharacter OtherActor)
  (Input|EnableInput (Game|GetPlayerController 0))
  (Utilities|FlowControl|Gate true) ; enters at Open
)

(event OnComponentEndOverlap(Green_Trigger)
  (params (OverlappedComponent :type Primitive%20Component%20Object%20Reference) (OtherActor :type Actor%20Object%20Reference) (OtherComp :type Primitive%20Component%20Object%20Reference) (OtherBodyIndex :type Integer))
  ;[1 1 1] Listen To Player
  (Utilities|Casting|CastToThirdPersonCharacter OtherActor)
  (Input|DisableInput (Game|GetPlayerController 0))
  (Utilities|FlowControl|Gate true) ; enters at Close
)

(event OnComponentBeginOverlap(Yellow_Trigger)
  (params (OverlappedComponent :type Primitive%20Component%20Object%20Reference) (OtherActor :type Actor%20Object%20Reference) (OtherComp :type Primitive%20Component%20Object%20Reference) (OtherBodyIndex :type Integer) (bFromSweep :type Boolean) (SweepResult :type Hit%20Result%20Structure%20%28by%20ref%29))
  ;[1 1 1] Listen To Player
  (Utilities|Casting|CastToThirdPersonCharacter OtherActor)
  (Input|EnableInput (Game|GetPlayerController 0))
  (Utilities|FlowControl|Gate true) ; enters at Open
)

(event OnComponentEndOverlap(Yellow_Trigger)
  (params (OverlappedComponent :type Primitive%20Component%20Object%20Reference) (OtherActor :type Actor%20Object%20Reference) (OtherComp :type Primitive%20Component%20Object%20Reference) (OtherBodyIndex :type Integer))
  ;[1 1 1] Listen To Player
  (Utilities|Casting|CastToThirdPersonCharacter OtherActor)
  (Input|DisableInput (Game|GetPlayerController 0))
  (Utilities|FlowControl|Gate true) ; enters at Close
)

(event OnComponentBeginOverlap(Blue_Trigger)
  (params (OverlappedComponent :type Primitive%20Component%20Object%20Reference) (OtherActor :type Actor%20Object%20Reference) (OtherComp :type Primitive%20Component%20Object%20Reference) (OtherBodyIndex :type Integer) (bFromSweep :type Boolean) (SweepResult :type Hit%20Result%20Structure%20%28by%20ref%29))
  ;[1 1 1] Listen To Player
  (Utilities|Casting|CastToThirdPersonCharacter OtherActor)
  (Input|EnableInput (Game|GetPlayerController 0))
  (Utilities|FlowControl|Gate true) ; enters at Open
)

(event OnComponentEndOverlap(Blue_Trigger)
  (params (OverlappedComponent :type Primitive%20Component%20Object%20Reference) (OtherActor :type Actor%20Object%20Reference) (OtherComp :type Primitive%20Component%20Object%20Reference) (OtherBodyIndex :type Integer))
  ;[1 1 1] Listen To Player
  (Utilities|Casting|CastToThirdPersonCharacter OtherActor)
  (Input|DisableInput (Game|GetPlayerController 0))
  (Utilities|FlowControl|Gate true) ; enters at Close
)

(event Custom|SetUp%20Dificulty
  ;[1 1 1] Set Up Difficulty
  (Utilities|Array|Clear (Variables|Default|GetPlayList))
  (switch int (Variables|Default|GetDifficulty)
    (:1
      (Variables|Default|SetNotesToRemember 4)
      (Variables|Default|SetSpeed 1.5))
    (:2
      (Variables|Default|SetNotesToRemember 4)
      (Variables|Default|SetSpeed 1.5))
    (:3
      (Variables|Default|SetNotesToRemember 5)
      (Variables|Default|SetSpeed 1.2))
    (:4
      (Variables|Default|SetNotesToRemember 6)
      (Variables|Default|SetSpeed 1.0))
    (:5
      (Variables|Default|SetNotesToRemember 7)
      (Variables|Default|SetSpeed 0.9))
    (:6
      (Variables|Default|SetNotesToRemember 8)
      (Variables|Default|SetSpeed 0.7))
    (:7
      (Variables|Default|SetNotesToRemember 9)
      (Variables|Default|SetSpeed 0.6))
    (:8
      (Variables|Default|SetNotesToRemember 10)
      (Variables|Default|SetSpeed 0.5))))

(event Custom|CreatePlayList
  ;[1 1 1] Add Note to Playlist
  (while (< (Utilities|Array|Length (Variables|Default|GetPlayList)) (Variables|Default|GetNotesToRemember))
    (Utilities|Array|Add (Variables|Default|GetPlayList) (Math|Random|RandomIntegerinRange 0 3)))
  (Utilities|FlowControl|Delay 1.0)
  (CallFunction|PlayPlaylist))

(event Custom|PlayPlaylist
  ;[1 1 1] Playplaylist
  (if (not (Variables|Default|GetisListening))
    (if (< (Variables|Default|GetNotesPlayed) (Variables|Default|GetNotesToRemember))
      (Variables|Default|SetisPlaying true)
      (switch int (Utilities|Array|Get(acopy) (Variables|Default|GetPlayList) (Variables|Default|GetNotesPlayed))
        (:0
          (CallFunction|CambiarColor false (Variables|Default|GetBlue_Light) 0 "(R=0.937500,G=0.937500,B=0.937500,A=1.000000)" "(R=0.105882,G=0.435294,B=0.729412,A=1.000000)"))
        (:1
          (CallFunction|CambiarColor false (Variables|Default|GetRed_Light) 0 "(R=0.947917,G=0.947917,B=0.947917,A=1.000000)" "(R=1.000000,G=0.027451,B=0.027451,A=1.000000)"))
        (:2
          (CallFunction|CambiarColor false (Variables|Default|GetGreen_Light) 0 "(R=0.869792,G=0.869792,B=0.869792,A=1.000000)" "(R=0.098039,G=0.572549,B=0.086275,A=1.000000)"))
        (:3
          (CallFunction|CambiarColor false (Variables|Default|GetYellow_Light) 0 "(R=0.864583,G=0.864583,B=0.864583,A=1.000000)" "(R=0.729412,G=0.686275,B=0.043137,A=1.000000)")))
      (Variables|Default|SetNotesPlayed (+ (Variables|Default|GetNotesPlayed) 1))
      (if (< (Variables|Default|GetNotesPlayed) (Variables|Default|GetNotesToRemember))
        (Utilities|FlowControl|Delay (Variables|Default|GetSpeed))
        (CallFunction|PlayPlaylist)
        (else
          (Variables|Default|SetisPlaying false)
          (Variables|Default|SetisListening true)))
      (else
        (Variables|Default|SetisListening true)))))

(event Custom|CambiarColor
  (params (IsFail :type Boolean) (Light :type Light%20Component%20Object%20Reference) (Sound :type Sound%20Base%20Object%20Reference) (ColorOff :type Linear%20Color%20Structure) (ColorOn :type Linear%20Color%20Structure))
  (bind _returnvalue (Transformation|GetWorldLocation Light))
  ;[1 1 1] PlayNotes
  (if IsFail
    (Audio|PlaySoundatLocation "/Game/Default/StarterContent/Audio/Collapse01.Collapse01" _returnvalue "0, 0, 0" (Variables|Default|GetVolume%20Multiplier) 1.0 0.0 0 0 0)
    (Rendering|Components|Light|SetLightColor (Variables|Default|GetYellow_Light) "(R=1.000000,G=0.027451,B=0.027451,A=1.000000)" true)
    (Utilities|FlowControl|Delay 1.0)
    (Rendering|Components|Light|SetLightColor (Variables|Default|GetYellow_Light) "(R=1.000000,G=0.932292,B=0.932292,A=1.000000)" true)
    (CallFunction|ResetSimon true)
    (else
      (Rendering|Components|Light|SetLightColor Light ColorOn true)
      (Audio|PlaySoundatLocation Sound _returnvalue "0, 0, 0" (Variables|Default|GetVolume%20Multiplier) 1.0 0.0 0 0 0)
      (Utilities|FlowControl|Delay (- (Variables|Default|GetSpeed) 0.2))
      (Rendering|Components|Light|SetLightColor Light ColorOff true))))

(event Custom|CheckWin
  ;[1 1 1] Check if player has won
  (if (== (Utilities|Array|Length (Variables|Default|GetPlayerPlaylist)) (Utilities|Array|Length (Variables|Default|GetPlayList)))
    (if (< (Variables|Default|GetDifficulty) (Variables|Default|GetMaxLevel))
      (Math|Integer|IncrementInt (Variables|Default|GetDifficulty)
        (:%20%20
          (CallFunction|ResetSimon false)))
      (else
        (Math|Integer|IncrementInt (Variables|Default|GetDifficulty)
          (:%20%20
            (Development|PrintString "YouWin")
            (CallFunction|ResetSimon false)))))))

(event Input|ActionEvents|InputActionUse
  (params (Key :type Key%20Structure :default "None"))
  ;[1 1 1] PlayerTrigger Overlap Events
  (:Pressed
    (if (not (or (Variables|Default|GetisPlaying) (Variables|Default|GetisListening)))
      (Utilities|FlowControl|Gate true
        (:Exit
          (CallFunction|SetUpDificulty)
          (CallFunction|CreatePlayList))))))

(event Input|ActionEvents|InputActionUse
  (params (Key :type Key%20Structure :default "None"))
  ;[1 1 1] Listen To Player
  (:Pressed
    (if (Variables|Default|GetisListening)
      (Utilities|FlowControl|Gate true
        (:Exit
          (bind _isfail (CallFunction|CheckNote))
          (CallFunction|CambiarColor _isfail (Variables|Default|GetBlue_Light) 0 "(R=0.937500,G=0.937500,B=0.937500,A=1.000000)" "(R=0.105882,G=0.435294,B=0.729412,A=1.000000)")
          (CallFunction|CheckWin))))))

(event Input|ActionEvents|InputActionUse
  (params (Key :type Key%20Structure :default "None"))
  ;[1 1 1] Listen To Player
  (:Pressed
    (if (Variables|Default|GetisListening)
      (Utilities|FlowControl|Gate true
        (:Exit
          (bind _isfail (CallFunction|CheckNote 1))
          (CallFunction|CambiarColor _isfail (Variables|Default|GetRed_Light) 0 "(R=0.947917,G=0.947917,B=0.947917,A=1.000000)" "(R=1.000000,G=0.027451,B=0.027451,A=1.000000)")
          (CallFunction|CheckWin))))))

(event Input|ActionEvents|InputActionUse
  (params (Key :type Key%20Structure :default "None"))
  ;[1 1 1] Listen To Player
  (:Pressed
    (if (Variables|Default|GetisListening)
      (Utilities|FlowControl|Gate true
        (:Exit
          (bind _isfail (CallFunction|CheckNote 2))
          (CallFunction|CambiarColor _isfail (Variables|Default|GetGreen_Light) 0 "(R=0.869792,G=0.869792,B=0.869792,A=1.000000)" "(R=0.098039,G=0.572549,B=0.086275,A=1.000000)")
          (CallFunction|CheckWin))))))

(event Input|ActionEvents|InputActionUse
  (params (Key :type Key%20Structure :default "None"))
  ;[1 1 1] Listen To Player
  (:Pressed
    (if (Variables|Default|GetisListening)
      (Utilities|FlowControl|Gate true
        (:Exit
          (bind _isfail (CallFunction|CheckNote 3))
          (CallFunction|CambiarColor _isfail (Variables|Default|GetYellow_Light) 0 "(R=0.864583,G=0.864583,B=0.864583,A=1.000000)" "(R=0.729412,G=0.686275,B=0.043137,A=1.000000)")
          (CallFunction|CheckWin))))))

(fn ConstructionScript)

(fn CheckNote
  (params (Note%20to%20Check :type Integer))
  (bind _playerplaylist (Variables|Default|GetPlayerPlaylist))
  (Utilities|Array|Add _playerplaylist Note%20to%20Check)
  (return (not (== Note%20to%20Check (Utilities|Array|Get(acopy) (Variables|Default|GetPlayList) (- (Utilities|Array|Length _playerplaylist) 1))))))

(fn ResetSimon
  (params (IsFail :type Boolean))
  (if IsFail
    (Variables|Default|SetisListening false)
    (Variables|Default|SetisPlaying false)
    (Utilities|Array|Clear (Variables|Default|GetPlayList))
    (Utilities|Array|Clear (Variables|Default|GetPlayerPlaylist))
    (Variables|Default|SetNotesToRemember 0)
    (Variables|Default|SetNotesPlayed 0)
    (Variables|Default|SetDifficulty 1)
    (else
      (Variables|Default|SetisListening false)
      (Variables|Default|SetisPlaying false)
      (Utilities|Array|Clear (Variables|Default|GetPlayList))
      (Utilities|Array|Clear (Variables|Default|GetPlayerPlaylist))
      (Variables|Default|SetNotesToRemember 0)
      (Variables|Default|SetNotesPlayed 0))))